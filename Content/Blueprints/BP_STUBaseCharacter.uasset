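; Base character Blueprint that feeds movement state to its mesh's animation instance.
; On BeginPlay it caches the anim instance if it implements AnimInterface_BaseCharacter.
; Every Tick, SetAnimData pushes speed, movement direction, falling and running state through interface messages, so the character needs no cast to a specific Anim Blueprint.
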(event EventBeginPlay
  (bind _mesh (Variables|Character|GetMesh))
  (bind _returnvalue (Components|SkeletalMesh|GetAnimInstance _mesh))
  (if (Utilities|DoesObjectImplementInterface _returnvalue "/Game/Blueprints/AnimInterface_BaseCharacter.AnimInterface_BaseCharacter_C")
    (Variables|Default|SetAInstance _returnvalue)))

(event EventTick
  (params (DeltaSeconds :type Float%20%28single-precision%29))
  (CallFunction|SetAnimData))

(fn ConstructionScript)

(fn SetAnimData
  (bind _ainstance (Variables|Default|GetAInstance))
  (Utilities|IsValid (Variables|Default|GetAInstance)
    (:Is%20Valid
      (Class|AnimInterfaceBaseCharacter|GetSpeed(Message) _ainstance (Class|STUBaseCharacter|GetSpeed))
      (Class|AnimInterfaceBaseCharacter|GetDirection(Message) _ainstance (Class|STUBaseCharacter|GetMovementDirection))
      (Class|AnimInterfaceBaseCharacter|IsFalling(Message) _ainstance (AI|Components|NavMovement|IsFalling (Variables|Character|GetCharacterMovement)))
      (Class|AnimInterfaceBaseCharacter|IsRunning(Message) _ainstance (Class|STUBaseCharacter|IsRunning)))))